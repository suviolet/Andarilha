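; BP_Car is a looping moving-car actor that repeatedly travels toward a Despawn component's position.
; After a random delay, it activates two Niagara effects and plays a timeline that moves the static mesh by scaling Despawn's relative location by Alpha.
; When the timeline ends, it deactivates the effects, waits, teleports the mesh to the location cached from StaticMesh1 at BeginPlay, then restarts the cycle.
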(event `SpawnCar`
  (`KismetSystemLibrary.Delay` (`KismetMathLibrary.RandomFloatInRange` 0.0 6.0))
  (`ActorComponent.Activate` (`self.Niagara`) false)
  (`ActorComponent.Activate` (`self.Niagara1`) false)
  (bind (_direction _alpha) (`Timeline|MoveCar` :`NewTime` (`self.Velocity`) :!via `PlayFromStart`)
    (:`Update`
      (`SceneComponent.K2_SetRelativeLocation` (`self.StaticMesh`) (* _alpha (`SceneComponent.RelativeLocation` (`self.Despawn`))) false false))
    (:`Finished`
      (`ActorComponent.Deactivate` (`self.Niagara`))
      (`ActorComponent.Deactivate` (`self.Niagara1`))
      (`KismetSystemLibrary.Delay` 2.0)
      (`SceneComponent.K2_SetRelativeLocation` (`self.StaticMesh`) (`self.StartLocation`) false true)
      (`self.SpawnCar`))))

(event `self.ReceiveBeginPlay`
  (set `self.StartLocation` (`SceneComponent.RelativeLocation` (`self.StaticMesh1`)))
  (`self.SpawnCar`))

(fn `UserConstructionScript`)