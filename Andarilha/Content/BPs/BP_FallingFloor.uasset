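; BP_FallingFloor is a floor trap that gives way shortly after the player character (BP_PCharacter) steps into its box trigger.
; It pairs a static mesh with a geometry collection, whose physics, gravity, collision damage and clustering are switched off on BeginPlay.
; After a short delay, the overlap destroys the mesh and turns on the collection's physics and clustering.
; Gravity and collision damage are never re-enabled in this Blueprint.
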(event `self.ReceiveBeginPlay`
  (bind _gc_fallingfloor (`self.GC_FallingFloor`))
  (`GeometryCollectionComponent.SetEnableDamageFromCollision` _gc_fallingfloor false)
  (set `GeometryCollectionComponent.EnableClustering` false _gc_fallingfloor)
  (`PrimitiveComponent.SetEnableGravity` _gc_fallingfloor false)
  (`PrimitiveComponent.SetSimulatePhysics` _gc_fallingfloor false))

(event `self.Box.OnComponentBeginOverlap`
  (params (OverlappedComponent :type "PrimitiveComponent Object Reference") (OtherActor :type "Actor Object Reference") (OtherComp :type "PrimitiveComponent Object Reference") (OtherBodyIndex :type Integer) (bFromSweep :type Boolean) (SweepResult :type "HitResult Structure (by ref)"))
  (bind _gc_fallingfloor (`self.GC_FallingFloor`))
  (cast `/Game/Characters/Andarilha/BP_PCharacter` OtherActor)
  (`KismetSystemLibrary.Delay` 1.0)
  (`ActorComponent.K2_DestroyComponent` (`self.StaticMesh`))
  (`PrimitiveComponent.SetSimulatePhysics` _gc_fallingfloor true)
  (set `GeometryCollectionComponent.EnableClustering` true _gc_fallingfloor))

(fn `UserConstructionScript`)