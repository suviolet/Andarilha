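; Level streaming trigger actor that loads or unloads a list of levels when the player character exits its box.
; On end overlap, the dot product of the character's forward vector and the Arrow's decides the action: positive loads, otherwise unloads.
; Load and unload events step through the Levels array by re-calling themselves after each blocking stream call, printing a message when done.
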(event `self.Box.OnComponentEndOverlap`
  (params (OverlappedComponent :type "PrimitiveComponent Object Reference") (OtherActor :type "Actor Object Reference") (OtherComp :type "PrimitiveComponent Object Reference") (OtherBodyIndex :type Integer))
  (bind _asbp_pcharacter (cast `/Game/Characters/Andarilha/BP_PCharacter` OtherActor))
  (set `self.index` 0)
  (if (> (`KismetMathLibrary.Dot_VectorVector` (`self.GetActorForwardVector` _asbp_pcharacter) (`SceneComponent.GetForwardVector` (`self.Arrow`))) 0.0)
    (`self.LoadLevel`)
    (else
      (`self.UnloadLevel`))))

(event `LoadLevel`
  (`GameplayStatics.LoadStreamLevel` (`|GetArrayItem` (`self.Levels`) (`self.index`)) true true)
  (if (< (`self.index`) (- (`KismetArrayLibrary.Array_Length` (`self.Levels`)) 1))
    (bind _result (`/Engine/EditorBlueprintResources/StandardMacros.IncrementInt` (`self.index`))
      (:`  `
        (set `self.index` _result)
        (`self.LoadLevel`)))
    (else
      (`KismetSystemLibrary.PrintString` "LOAD DONE"))))

(event `UnloadLevel`
  (`GameplayStatics.UnloadStreamLevel` (`|GetArrayItem` (`self.Levels`) (`self.index`)) true)
  (if (< (`self.index`) (- (`KismetArrayLibrary.Array_Length` (`self.Levels`)) 1))
    (bind _result (`/Engine/EditorBlueprintResources/StandardMacros.IncrementInt` (`self.index`))
      (:`  `
        (set `self.index` _result)
        (`self.UnloadLevel`)))
    (else
      (`KismetSystemLibrary.PrintString` "UNLOAD DONE"))))

(fn `UserConstructionScript`)