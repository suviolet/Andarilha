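; BP_SecurityCameraOnlyFollows is a security camera actor that turns to follow the player character, with no other behavior.
; A Box trigger stores the overlapping BP_PCharacter as Player and sets IsOnSight, which clears when that character leaves.
; While IsOnSight is true, Tick snaps CameraMain's world rotation to face the player's location, without interpolation.
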(event `self.ReceiveTick`
  (params (DeltaSeconds :type "Float (single-precision)"))
  (if (`self.bIsOnSight`)
    (`SceneComponent.K2_SetWorldRotation` (`self.CameraMain`) (`KismetMathLibrary.Conv_VectorToRotator` (- (`self.K2_GetActorLocation` (`self.Player`)) (`SceneComponent.K2_GetComponentLocation` (`self.CameraMain`)))) false false)))

(event `self.Box.OnComponentBeginOverlap`
  (params (OverlappedComponent :type "PrimitiveComponent Object Reference") (OtherActor :type "Actor Object Reference") (OtherComp :type "PrimitiveComponent Object Reference") (OtherBodyIndex :type Integer) (bFromSweep :type Boolean) (SweepResult :type "HitResult Structure (by ref)"))
  (bind _asbp_pcharacter (cast `/Game/Characters/Andarilha/BP_PCharacter` OtherActor))
  (set `self.Player` _asbp_pcharacter)
  (set `self.bIsOnSight` true))

(event `self.Box.OnComponentEndOverlap`
  (params (OverlappedComponent :type "PrimitiveComponent Object Reference") (OtherActor :type "Actor Object Reference") (OtherComp :type "PrimitiveComponent Object Reference") (OtherBodyIndex :type Integer))
  (cast `/Game/Characters/Andarilha/BP_PCharacter` OtherActor)
  (set `self.bIsOnSight` false))

(fn `UserConstructionScript`)