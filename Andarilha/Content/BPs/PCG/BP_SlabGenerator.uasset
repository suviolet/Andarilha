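; BP_SlabGenerator is an unfinished procedural generator meant to build a slab from its construction script.
; GenerateSlab loops XCount up to XRows, spawning a plain Actor each pass at the generator's own transform, with no offset between copies.
; The node that resets XCount to zero is disconnected, and the event graph is empty.
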(event `self.ReceiveBeginPlay`)

(event `self.ReceiveTick`
  (params (DeltaSeconds :type "Float (single-precision)")))

(fn `GenerateSlab`
  (while (< (`self.XCount`) (`self.XRows`))
    (`|SpawnActorFromClass` (`self.Actor`) (`self.GetTransform`) "Undefined" "MultiplyWithRoot" null null)
    (`/Engine/EditorBlueprintResources/StandardMacros.IncrementInt` (`self.XCount`))))

(fn `UserConstructionScript`
  (`self.GenerateSlab`))